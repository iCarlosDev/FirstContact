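; EnemyAttach is an actor that moves relative to placed EnemyAttack points, driven by the third-person character's Position value.
; BeginPlay caches the character and stores two EnemyAttack locations, split by whether EnemyINT is zero.
; Each Tick, ChooseEnemyAttack selects the point, and a swept move lerps between it and the current location using Position as alpha.
; The second branch reverses the lerp inputs, so Position pulls the opposite way.
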(event `self.ReceiveBeginPlay`
  (`|ExecutionSequence`
    (:`then_0`
      (bind _returnvalue (`GameplayStatics.GetActorOfClass` "/Game/ThirdPerson/Blueprints/BP_ThirdPersonCharacter.BP_ThirdPersonCharacter_C"))
      (set `self.ThirdPersonCharacter` _returnvalue))
    (:`then_1`
      (bind _outactors (`GameplayStatics.GetAllActorsOfClass` "/Game/Members/Carlos/Blueprints/EnemyAttack.EnemyAttack_C"))
      (for _array_element _outactors
        (if (== (`/Game/Members/Carlos/Blueprints/EnemyAttack.EnemyINT` _array_element) 0)
          (bind _returnvalue_2 (`self.K2_GetActorLocation` _array_element))
          (set `self.Location1` _returnvalue_2)
          (else
            (set `self.Location2` _returnvalue_2)))))))

(event `self.ReceiveTick`
  (params (DeltaSeconds :type "Float (single-precision)"))
  (bind _position (`/Game/ThirdPerson/Blueprints/BP_ThirdPersonCharacter.Position` (`self.ThirdPersonCharacter`)))
  (if (== (`self.ChooseEnemyAttack`) 0)
    (`self.K2_SetActorLocation` (`KismetMathLibrary.VLerp` (`self.K2_GetActorLocation`) (`self.Location1`) _position) true)
    (else
      (`self.K2_SetActorLocation` (`KismetMathLibrary.VLerp` (`self.Location2`) (`self.K2_GetActorLocation`) _position) true))))

(fn `UserConstructionScript`)